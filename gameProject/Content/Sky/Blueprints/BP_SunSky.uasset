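; BP_SunSky is a sky Blueprint that drives a day-night cycle.
; Each Tick calls the parent logic, then advances SolarTime by delta seconds scaled by TimeMultiplier, wrapping it at 24 hours.
; IsNight reports whether SolarTime falls in the night window between StartOfNight and EndOfNight, which spans midnight.
; The construction script only defers to its parent.
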(event EventBeginPlay)

(event Collision|EventActorBeginOverlap
  (params (OtherActor :type Actor%20Object%20Reference)))

(event EventTick
  (params (DeltaSeconds :type Float%20%28single-precision%29))
  ;[1 0.6584 0.25] Day-Night Cycle
  (|CallParentFunction DeltaSeconds)
  (Variables|Default|SetSolarTime (Math|Float|%(Float) (+ (* DeltaSeconds (Variables|Default|GetTimeMultiplier)) (Variables|Default|GetSolarTime)) 24.0)))

(fn ConstructionScript
  (|CallParentFunction))

(fn IsNight
  (return (or (>= (Variables|Default|GetSolarTime) (Variables|Default|GetStartOfNight)) (< (Variables|Default|GetSolarTime) (Variables|Default|GetEndOfNight)))))