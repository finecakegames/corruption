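; BP_Moons is a sky actor with a main moon and a sub moon, each given its own dynamic instance of M_Moon.
; The construction script creates and assigns both instances, overriding the Color parameter on the sub moon with a dark olive tint.
; Tick sets the sub moon's relative rotation on all axes to scaled delta time, an absolute value that does not accumulate into a continuous spin.
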(event EventBeginPlay)

(event Collision|EventActorBeginOverlap
  (params (OtherActor :type Actor%20Object%20Reference)))

(event EventTick
  (params (DeltaSeconds :type Float%20%28single-precision%29))
  (bind _returnvalue (* DeltaSeconds 1e+01))
  (Transformation|SetRelativeRotation (Variables|Default|GetSubMoon) (Math|Rotator|MakeRotator _returnvalue _returnvalue _returnvalue) false false))

(fn ConstructionScript
  (bind _mainmoon (Variables|Default|GetMainMoon))
  (bind _submoon (Variables|Default|GetSubMoon))
  (bind _returnvalue (Rendering|Material|CreateDynamicMaterialInstance _mainmoon 0 "/Game/Sky/M_Moon.M_Moon" "M_MainMoon" :!class /Script/Engine.PrimitiveComponent))
  (Rendering|Material|SetMaterial _mainmoon 0 _returnvalue)
  (bind _returnvalue_2 (Rendering|Material|CreateDynamicMaterialInstance _submoon 0 "/Game/Sky/M_Moon.M_Moon" "M_SubMoon" :!class /Script/Engine.PrimitiveComponent))
  (Rendering|Material|SetVectorParameterValueonMaterials (Variables|Default|GetSubMoon) "Color" (Math|Conversions|ToVector(LinearColor) "(R=0.126430,G=0.151042,B=0.079454,A=1.000000)"))
  (Rendering|Material|SetMaterial _submoon 0 _returnvalue_2))