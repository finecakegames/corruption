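; PowerupManager applies timed Damage and Speed power-ups to the player's BP_MainCharacter.
; AddPowerUp looks up the item's type, raises damage or walk and crouch speeds, and sets a 30-second countdown in the ActivePowerups map.
; A looping one-second timer prints and decrements each countdown, calling RemovePowerUp at zero to subtract the boost.
; Re-adding an active item resets its countdown but applies the boost again.
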(event EventBeginPlay
  (Utilities|Time|SetTimerbyFunctionName 0 "TickPowerUps" 1.0 true))

(event EventTick
  (params (DeltaSeconds :type Float%20%28single-precision%29)))

(fn TickPowerUps
  (bind _activepowerups (Variables|Default|GetActivePowerups))
  (bind _keys (Utilities|Map|Keys _activepowerups))
  (for _array_element _keys
    (Development|PrintText (Utilities|Text|FormatText "PowerUp : {1} -- {0}" _array_element (Utilities|Text|ToText(Integer) (.Value (Utilities|Map|Find _activepowerups _array_element)))))
    (if (== (- (.Value (Utilities|Map|Find _activepowerups _array_element)) 1) 0)
      (CallFunction|RemovePowerUp _array_element)
      (else
        (Utilities|Map|Add _activepowerups _array_element (- (.Value (Utilities|Map|Find _activepowerups _array_element)) 1))))))

(fn RemovePowerUp
  (params (ConsumableID :type Name))
  (bind _poweruptypes (Variables|Default|GetPowerUpTypes))
  (bind (_value _returnvalue) (Utilities|Map|Find _poweruptypes ConsumableID))
  (if _returnvalue
    (bind _asbp_main_character (Utilities|Casting|CastToBP_MainCharacter (Game|GetPlayerCharacter 0)))
    (Variables|Default|SetCharacter _asbp_main_character)
    (switch name _value
      (:damage
        (Variables|/Game/Characters/MainCharacter/Blueprints/BP_MainCharacter.BP_MainCharacter_C|SetDamage (Variables|Default|GetCharacter) (- (Variables|/Game/Characters/MainCharacter/Blueprints/BP_MainCharacter.BP_MainCharacter_C|GetDamage (Variables|Default|GetCharacter)) (Variables|Default|GetDamageBoost))))
      (:speed
        (Variables|/Script/Engine.CharacterMovementComponent|SetMaxWalkSpeed (Variables|/Script/Engine.Character|GetCharacterMovement (Variables|Default|GetCharacter)) (- (Variables|/Script/Engine.CharacterMovementComponent|GetMaxWalkSpeed (Variables|/Script/Engine.Character|GetCharacterMovement (Variables|Default|GetCharacter))) (Variables|Default|GetSpeedBoost)))
        (Variables|/Script/Engine.CharacterMovementComponent|SetMaxWalkSpeedCrouched (Variables|/Script/Engine.Character|GetCharacterMovement (Variables|Default|GetCharacter)) (/ (- (Variables|/Script/Engine.CharacterMovementComponent|GetMaxWalkSpeed (Variables|/Script/Engine.Character|GetCharacterMovement (Variables|Default|GetCharacter))) (Variables|Default|GetSpeedBoost)) 2.0))))
    (Utilities|Map|Remove (Variables|Default|GetActivePowerups) ConsumableID)))

(fn AddPowerUp
  (params (ItemID :type Name))
  (bind _poweruptypes (Variables|Default|GetPowerUpTypes))
  (bind (_value _returnvalue) (Utilities|Map|Find _poweruptypes ItemID))
  (if _returnvalue
    (bind _asbp_main_character (Utilities|Casting|CastToBP_MainCharacter (Game|GetPlayerCharacter 0)))
    (LocalVariables|SetCharacter _asbp_main_character)
    (switch name _value
      (:damage
        (Variables|/Game/Characters/MainCharacter/Blueprints/BP_MainCharacter.BP_MainCharacter_C|SetDamage (LocalVariables|GetCharacter) (+ (Variables|/Game/Characters/MainCharacter/Blueprints/BP_MainCharacter.BP_MainCharacter_C|GetDamage (LocalVariables|GetCharacter)) (Variables|Default|GetDamageBoost))))
      (:speed
        (Variables|/Script/Engine.CharacterMovementComponent|SetMaxWalkSpeed (Variables|/Script/Engine.Character|GetCharacterMovement (LocalVariables|GetCharacter)) (+ (Variables|/Script/Engine.CharacterMovementComponent|GetMaxWalkSpeed (Variables|/Script/Engine.Character|GetCharacterMovement (LocalVariables|GetCharacter))) (Variables|Default|GetSpeedBoost)))
        (Variables|/Script/Engine.CharacterMovementComponent|SetMaxWalkSpeedCrouched (Variables|/Script/Engine.Character|GetCharacterMovement (LocalVariables|GetCharacter)) (/ (+ (Variables|/Script/Engine.CharacterMovementComponent|GetMaxWalkSpeed (Variables|/Script/Engine.Character|GetCharacterMovement (LocalVariables|GetCharacter))) (Variables|Default|GetSpeedBoost)) 2.0))))
    (Utilities|Map|Add (Variables|Default|GetActivePowerups) ItemID 30)))