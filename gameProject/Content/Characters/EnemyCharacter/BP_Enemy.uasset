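; Enemy character that detects, attacks and takes damage from the player character.
; Pawn sensing sets the AI blackboard's playerInSight flag on seeing the player; this file never clears it.
; AttackPlayer sphere-traces forward with debug drawing and damages a hit player, with no montage asset specified.
; Incoming damage passes a DoOnce that resets after the hit-montage delay, ignoring hits meanwhile, and destroys the enemy at zero health.
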(event OnSeePawn(PawnSensing)
  (params (Pawn :type Pawn%20Object%20Reference))
  (Utilities|Casting|CastToBP_MainCharacter Pawn)
  (AI|Components|Blackboard|SetValueasBool (AI|GetBlackboard (AI|GetAIController self)) (Utilities|Name|MakeLiteralName "playerInSight") true))

(event OnHearNoise(PawnSensing)
  (params (Instigator :type Pawn%20Object%20Reference) (Location :type Vector%20%28by%20ref%29 :default "0, 0, 0") (Volume :type Float%20%28single-precision%29)))

(event Custom|AttackPlayer
  (bind _returnvalue (Transformation|GetActorLocation))
  (bind (_outhit _returnvalue_2) (Collision|SphereTraceForObjects _returnvalue (+ _returnvalue (* 2.5e+02 (Math|Vector|GetForwardVector (Transformation|GetActorRotation)))) (Variables|Default|GetHitRadius) (Utilities|Array|MakeArray "ObjectTypeQuery3") false 0 "ForDuration"))
  (if _returnvalue_2
    (bind _asbp_main_character (Utilities|Casting|CastToBP_MainCharacter (.HitActor (Collision|BreakHitResult _outhit))))
    ;[0.05098 0.05098 0.05098 1 14] TODO
    (Animation|PlayAnimMontage 0 1.0 "None")
    (Game|Damage|ApplyDamage _asbp_main_character 1e+01 0 0 "/Script/Engine.DamageType")))

(event EventBeginPlay)

(event Collision|EventActorBeginOverlap
  (params (OtherActor :type Actor%20Object%20Reference)))

(event EventTick
  (params (DeltaSeconds :type Float%20%28single-precision%29)))

(event Game|Damage|EventAnyDamage
  (params (Damage :type Float%20%28single-precision%29) (DamageType :type Damage%20Type%20Object%20Reference) (InstigatedBy :type Controller%20Object%20Reference) (DamageCauser :type Actor%20Object%20Reference))
  ;[0.4375 0.03646 0.04047] Taking Damage
  (Utilities|FlowControl|DoOnce false :!label _label
    (:Completed
      (bind _output_get (Variables|Default|SetHealth (- (Variables|Default|GetHealth) Damage)))
      (if (<= _output_get 0.0)
        (Actor|DestroyActor)
        (Development|PrintText "MONSTER DEAD")
        (else
          (bind _returnvalue (Animation|PlayAnimMontage 0 1.0 "None"))
          (Utilities|FlowControl|Delay _returnvalue)
          (goto _label Reset))))))

(fn ConstructionScript)