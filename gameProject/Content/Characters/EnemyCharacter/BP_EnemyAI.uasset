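; Enemy character Blueprint that detects the player by sight and performs a melee-style attack check.
; Pawn sensing flags playerInSight on the AI controller's blackboard when it sees an FPCharacter, and nothing here clears it.
; AttackPlayer sphere-traces forward for pawns with debug drawing, then calls PlayAnimMontage on an FPCharacter hit, with no montage set or damage applied.
; Noise sensing is unimplemented.
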(event OnSeePawn(PawnSensing)
  (params (Pawn :type Pawn%20Object%20Reference))
  (Utilities|Casting|CastToFPCharacter Pawn)
  (AI|Components|Blackboard|SetValueasBool (AI|GetBlackboard (AI|GetAIController self)) (Utilities|Name|MakeLiteralName "playerInSight") true))

(event OnHearNoise(PawnSensing)
  (params (Instigator :type Pawn%20Object%20Reference) (Location :type Vector%20%28by%20ref%29 :default "0, 0, 0") (Volume :type Float%20%28single-precision%29)))

(event Custom|AttackPlayer
  (bind _returnvalue (Transformation|GetActorLocation))
  (bind (_outhit _returnvalue_2) (Collision|SphereTraceForObjects _returnvalue (+ _returnvalue (* 2.5e+02 (Math|Vector|GetForwardVector (Transformation|GetActorRotation)))) 1.2e+02 (Utilities|Array|MakeArray "ObjectTypeQuery3") false 0 "ForDuration"))
  (if _returnvalue_2
    (Utilities|Casting|CastToFPCharacter (.HitActor (Collision|BreakHitResult _outhit)))
    (Animation|PlayAnimMontage 0 1.0 "None")))

(event EventBeginPlay)

(event Collision|EventActorBeginOverlap
  (params (OtherActor :type Actor%20Object%20Reference)))

(event EventTick
  (params (DeltaSeconds :type Float%20%28single-precision%29)))

(fn ConstructionScript)