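; BP_Monster is an enemy character that takes damage and deals melee damage to BP_MainCharacter.
; A dynamic material instance made in the construction script lets hits tint the mesh red.
; A DoOnce gates health loss, sound and hit montage, resetting after a short delay, while death destroys the actor.
; AttackPlayer runs a sphere overlap at AttackSphere and applies damage to each player character found.
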(event Custom|AttackPlayer
  ;[1 1 1] Attack Player
  (bind _outactors (Collision|SphereOverlapActors (Transformation|GetWorldLocation (Variables|Default|GetAttackSphere)) (Variables|Default|GetAttackSphereRadius) (Utilities|Array|MakeArray "ObjectTypeQuery3") "/Game/Characters/MainCharacter/Blueprints/BP_MainCharacter.BP_MainCharacter_C" (Utilities|Array|MakeArray self)))
  (for _array_element _outactors
    (Game|Damage|ApplyDamage _array_element (Variables|Default|GetDamage) (Pawn|GetController) self "/Script/Engine.DamageType")))

(event Game|Damage|EventAnyDamage
  (params (Damage :type Float%20%28single-precision%29) (DamageType :type Damage%20Type%20Object%20Reference) (InstigatedBy :type Controller%20Object%20Reference) (DamageCauser :type Actor%20Object%20Reference))
  ;[0.4375 0.03646 0.04047] Taking Damage
  (Rendering|Material|SetVectorParameterValue (Variables|Default|GetMaterial) "InflictedDamageColor" "(R=0.572917,G=0.000000,B=0.000000,A=1.000000)" :!class /Script/Engine.MaterialInstanceDynamic)
  (Utilities|FlowControl|DoOnce false :!label _label
    (:Completed
      (Audio|PlaySound2D "/Game/Sounds/Effects/Punch.Punch" 1.0 1.0 0.0 0 0)
      (bind _output_get (Variables|Default|SetHealth (- (Variables|Default|GetHealth) Damage)))
      (if (<= _output_get 0.0)
        (Actor|DestroyActor)
        (Development|PrintText "MONSTER DEAD")
        (else
          (Animation|PlayAnimMontage 0 1.0 "None")
          (Utilities|FlowControl|Delay 0.5)
          (Rendering|Material|SetVectorParameterValue (Variables|Default|GetMaterial) "InflictedDamageColor" "(R=0.000000,G=0.000000,B=0.000000,A=1.000000)" :!class /Script/Engine.MaterialInstanceDynamic)
          (goto _label Reset))))))

(fn ConstructionScript
  (bind _mesh (Variables|Character|GetMesh))
  (bind _returnvalue (Rendering|Material|CreateDynamicMaterialInstance _mesh 0 (Rendering|Material|GetMaterial _mesh 0) "None" :!class /Script/Engine.PrimitiveComponent))
  (Rendering|Material|SetMaterial (Variables|Character|GetMesh) 0 _returnvalue)
  (Variables|Default|SetMaterial _returnvalue))