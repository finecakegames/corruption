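; BP_LevelStreamer is an overlap trigger that moves the player from one streamed level to the next.
; When BP_MainCharacter overlaps it, input is disabled and a WB_ChangeLevel widget covers the non-blocking load of LevelToLoad.
; The player is then teleported to the NewLevelPosition component, the widget is removed and input restored.
; Finally, PreviousLevel is unloaded without blocking.
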(event EventBeginPlay)

(event Collision|EventActorBeginOverlap
  (params (OtherActor :type Actor%20Object%20Reference))
  (bind _returnvalue (Game|GetPlayerCharacter 0))
  (bind _asbp_main_character (Utilities|Casting|CastToBP_MainCharacter OtherActor))
  (Input|DisableInput _asbp_main_character (Game|GetPlayerController 0))
  (bind _returnvalue_2 (UserInterface|CreateWidget "/Game/Levels/WB_ChangeLevel.WB_ChangeLevel_C"))
  (UserInterface|Viewport|AddtoViewport _returnvalue_2 0)
  (Class|GameplayStatics|LoadStreamLevelbySoftObjectPtr (Variables|Default|GetLevelToLoad) true false)
  (Transformation|SetActorLocation _returnvalue (Transformation|GetWorldLocation (Variables|Default|GetNewLevelPosition)) false true)
  (Widget|RemovefromParent _returnvalue_2)
  (Input|EnableInput _returnvalue (Game|GetPlayerController 0))
  (Class|GameplayStatics|UnloadStreamLevelbySoftObjectPtr (Variables|Default|GetPreviousLevel) false))

(fn ConstructionScript)